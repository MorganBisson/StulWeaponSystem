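; BP_StulWeapon is a test weapon Blueprint that prints debug messages for reload events.
; On BeginPlay it binds handlers to the reload started, cancelled and completed events, each printing its state.
; The completed handler also prints values labeled current and max ammo, read as gameplay attributes from the AbilitySystemComponent.
; An authority-gated initialization from the DA_WeaponTest definition is present but never runs.
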(event Custom|OnReloadCompleted_Event
  (params (Weapon :type Stul%20Weapon%20Object%20Reference))
  (Development|PrintString "Reload Completed")
  (Development|PrintString (Utilities|String|Append (Utilities|String|MakeLiteralString "Current Ammo: ") (Utilities|String|ToString(Float) (.ReturnValue (Class|AbilitySystemComponent|GetGameplayAttributeValue (Variables|Default|GetAbilitySystemComponent) "(AttributeName=\"CurrentAmmo\",Attribute=/Script/StulWeaponSystem.StulWeaponAttributeSet:CurrentAmmo,AttributeOwner=\"/Script/CoreUObject.Class'/Script/StulWeaponSystem.StulWeaponAttributeSet'\")")))))
  (Development|PrintString (Utilities|String|Append (Utilities|String|MakeLiteralString "Max Ammo: ") (Utilities|String|ToString(Float) (.ReturnValue (Class|AbilitySystemComponent|GetGameplayAttributeValue (Variables|Default|GetAbilitySystemComponent) "(AttributeName=\"MaxAmmo\",Attribute=/Script/Boston_Project.WeaponAttributeSet:MaxAmmo,AttributeOwner=\"/Script/CoreUObject.Class'/Script/Boston_Project.WeaponAttributeSet'\")"))))))

(event Custom|OnReloadStarted_Event
  (params (Weapon :type Stul%20Weapon%20Object%20Reference))
  (Development|PrintString "Reload Started"))

(event Custom|OnReloadCancelled_Event
  (params (Weapon :type Stul%20Weapon%20Object%20Reference))
  (Development|PrintString "Reload Cancelled"))

(event EventBeginPlay
  (EventDispatchers|BindEventtoOnReloadCompleted (delegate Custom|OnReloadCompleted_Event))
  (EventDispatchers|BindEventtoOnReloadStarted (delegate Custom|OnReloadStarted_Event))
  (EventDispatchers|BindEventtoOnReloadCancelled (delegate Custom|OnReloadCancelled_Event)))

(fn ConstructionScript)