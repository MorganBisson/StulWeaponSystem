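; BP_StulTestCharacter is a test player character that exercises the Stul weapon system through Enhanced Input.
; Possession initializes the StulWeaponManager's default loadout, and newly equipped weapons snap to the WeaponAttach0 component.
; Fire, aim, reload and fire-mode inputs reach the manager as gameplay tags, while slot equip and holster call it directly.
; It supplies the camera transform as weapon view data and provides no movement data.
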(event OnWeaponEquipped(StulWeaponManager)
  (params (NewWeapon :type Stul%20Weapon%20Object%20Reference) (PreviousWeapon :type Stul%20Weapon%20Object%20Reference))
  (Transformation|AttachComponentToComponent NewWeapon (Variables|Default|GetWeaponAttach_0) "None" "SnapToTarget" "SnapToTarget" "KeepRelative" true))

(event Input|EnhancedActionEvents|EnhancedInputActionIA_Move
  (params (ActionValue :type Vector%202D%20Structure) (ElapsedSeconds :type Float%20%28double-precision%29) (TriggeredSeconds :type Float%20%28double-precision%29) (InputAction :type Input%20Action%20Object%20Reference :default "/Game/FirstPerson/Input/Actions/IA_Move.IA_Move"))
  (bind (_x _y) (Math|Vector2D|BreakVector2D ActionValue))
  (Pawn|Input|AddMovementInput (Transformation|GetActorForwardVector) _y false)
  (Pawn|Input|AddMovementInput (Transformation|GetActorRightVector) _x false))

(event Input|EnhancedActionEvents|EnhancedInputActionIA_Look
  (params (ActionValue :type Vector%202D%20Structure) (ElapsedSeconds :type Float%20%28double-precision%29) (TriggeredSeconds :type Float%20%28double-precision%29) (InputAction :type Input%20Action%20Object%20Reference :default "/Game/FirstPerson/Input/Actions/IA_Look.IA_Look"))
  (bind (_x _y) (Math|Vector2D|BreakVector2D ActionValue))
  (Pawn|Input|AddControllerYawInput _x)
  (Pawn|Input|AddControllerPitchInput _y))

(event Input|EnhancedActionEvents|EnhancedInputActionIA_Shoot
  (params (ActionValue :type Boolean) (ElapsedSeconds :type Float%20%28double-precision%29) (TriggeredSeconds :type Float%20%28double-precision%29) (InputAction :type Input%20Action%20Object%20Reference :default "/Game/FirstPerson/Input/Actions/IA_Shoot.IA_Shoot"))
  (bind _stulweaponmanager (Variables|Default|GetStulWeaponManager))
  ;[0 0 0 0.5] Weapon Inputs
  (:Started
    (Class|StulWeaponManagerComponent|InputTagPressed _stulweaponmanager "(TagName=\"Stul.Weapon.Input.Fire\")"))
  (:Canceled
    (Class|StulWeaponManagerComponent|InputTagReleased _stulweaponmanager "(TagName=\"Stul.Weapon.Input.Fire\")" :!label _label))
  (:Completed
    (goto _label)))

(event Input|EnhancedActionEvents|EnhancedInputActionIA_Aim
  (params (ActionValue :type Boolean) (ElapsedSeconds :type Float%20%28double-precision%29) (TriggeredSeconds :type Float%20%28double-precision%29) (InputAction :type Input%20Action%20Object%20Reference :default "/Game/FirstPerson/Input/Actions/Weapon/IA_Aim.IA_Aim"))
  (bind _stulweaponmanager (Variables|Default|GetStulWeaponManager))
  ;[0 0 0 0.5] Weapon Inputs
  (:Started
    (Class|StulWeaponManagerComponent|InputTagPressed _stulweaponmanager "(TagName=\"Stul.Weapon.Input.Aim\")"))
  (:Canceled
    (Class|StulWeaponManagerComponent|InputTagReleased _stulweaponmanager "(TagName=\"Stul.Weapon.Input.Aim\")" :!label _label))
  (:Completed
    (goto _label)))

(event Input|EnhancedActionEvents|EnhancedInputActionIA_EquipPrimary
  (params (ActionValue :type Boolean) (ElapsedSeconds :type Float%20%28double-precision%29) (TriggeredSeconds :type Float%20%28double-precision%29) (InputAction :type Input%20Action%20Object%20Reference :default "/Game/FirstPerson/Input/Actions/Weapon/IA_EquipPrimary.IA_EquipPrimary"))
  ;[0 0 0 0.5] Weapon Inputs
  (:Started
    (Class|StulWeaponManagerComponent|EquipWeaponatSlot (Variables|Default|GetStulWeaponManager))))

(event Input|EnhancedActionEvents|EnhancedInputActionIA_EquipSecondary
  (params (ActionValue :type Boolean) (ElapsedSeconds :type Float%20%28double-precision%29) (TriggeredSeconds :type Float%20%28double-precision%29) (InputAction :type Input%20Action%20Object%20Reference :default "/Game/FirstPerson/Input/Actions/Weapon/IA_EquipSecondary.IA_EquipSecondary"))
  ;[0 0 0 0.5] Weapon Inputs
  (:Started
    (Class|StulWeaponManagerComponent|EquipWeaponatSlot (Variables|Default|GetStulWeaponManager) 1)))

(event Input|EnhancedActionEvents|EnhancedInputActionIA_HolsterWeapon
  (params (ActionValue :type Boolean) (ElapsedSeconds :type Float%20%28double-precision%29) (TriggeredSeconds :type Float%20%28double-precision%29) (InputAction :type Input%20Action%20Object%20Reference :default "/Game/FirstPerson/Input/Actions/Weapon/IA_HolsterWeapon.IA_HolsterWeapon"))
  ;[0 0 0 0.5] Weapon Inputs
  (:Started
    (Class|StulWeaponManagerComponent|HolsterWeapon (Variables|Default|GetStulWeaponManager))))

(event Input|EnhancedActionEvents|EnhancedInputActionIA_ChangeShootingMode
  (params (ActionValue :type Boolean) (ElapsedSeconds :type Float%20%28double-precision%29) (TriggeredSeconds :type Float%20%28double-precision%29) (InputAction :type Input%20Action%20Object%20Reference :default "/Game/FirstPerson/Input/Actions/Weapon/IA_ChangeShootingMode.IA_ChangeShootingMode"))
  ;[0 0 0 0.5] Weapon Inputs
  (:Started
    (Class|StulWeaponManagerComponent|InputTagPressed (Variables|Default|GetStulWeaponManager) "(TagName=\"Stul.Weapon.Input.ChangeFireMode\")")))

(event Input|EnhancedActionEvents|EnhancedInputActionIA_Reload
  (params (ActionValue :type Boolean) (ElapsedSeconds :type Float%20%28double-precision%29) (TriggeredSeconds :type Float%20%28double-precision%29) (InputAction :type Input%20Action%20Object%20Reference :default "/Game/FirstPerson/Input/Actions/IA_Reload.IA_Reload"))
  ;[0 0 0 0.5] Weapon Inputs
  (:Started
    (Class|StulWeaponManagerComponent|InputTagPressed (Variables|Default|GetStulWeaponManager) "(TagName=\"Stul.Weapon.Input.Reload\")")))

(event EventPossessed
  (params (NewController :type Controller%20Object%20Reference))
  (Class|StulWeaponManagerComponent|InitializeDefaultLoadout (Variables|Default|GetStulWeaponManager)))

(fn ConstructionScript)

(fn GetWeaponMovementData
  (return "" false))

(fn GetWeaponViewData
  (bind _camera (Variables|Default|GetCamera))
  (return (Utilities|Struct|MakeStulWeaponViewData (Transformation|GetWorldLocation _camera) (Transformation|GetWorldRotation _camera)) true))